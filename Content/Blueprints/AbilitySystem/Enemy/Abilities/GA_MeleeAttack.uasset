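; Enemy melee attack ability that plays a random tagged montage facing the combat target and damages players near the striking socket.
; On the montage's tagged gameplay event, it sphere-checks live players around that socket, filtering non-enemies unless the avatar has friendly fire.
; A hit executes the MeleeImpact gameplay cue with the montage tag, and the ability ends after the strike or when the montage finishes or is interrupted.
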(event Ability|EventActivateAbility
  (bind _returnvalue (Ability|GetAvatarActorfromActorInfo))
  (Variables|Default|SetHasHitTarget false)
  (bind _returnvalue_2 (Class|EnemyInterface|GetCombatTarget(Message) _returnvalue))
  (bind _output_get (Variables|Default|SetCombatTarget _returnvalue_2))
  (bind _ascombat_interface (Utilities|Casting|CastToCombatInterface _returnvalue))
  (Class|CombatInterface|UpdateFacingTarget _ascombat_interface (Transformation|GetActorLocation _output_get))
  (bind _output_get_2 (Variables|Default|SetAvatarActor (Ability|GetAvatarActorfromActorInfo)))
  (bind _returnvalue_3 (Class|CombatInterface|GetAttackMontages(Message) _output_get_2))
  (bind _output_get_3 (Variables|Default|SetTaggedMontage (Class|AuraDamageGameplayAbility|GetRandomTaggedMontage _returnvalue_3)))
  (|PlayMontageandWaitProxy "None" (.Montage (Utilities|Struct|BreakTaggedMontage _output_get_3)) 1.0 "None" false 1.0 0.0 false
    (:then
      (Ability|Tasks|WaitGameplayEvent (.MontageTag (Utilities|Struct|BreakTaggedMontage _output_get_3)) 0
        (:EventReceived
          (bind _returnvalue_4 (Class|CombatInterface|GetCombatSocketPos(Message) (Variables|Default|GetAvatarActor) (.SocketTag (Utilities|Struct|BreakTaggedMontage _output_get_3))))
          (bind _output_get_4 (Variables|Default|SetCombatSocketPos _returnvalue_4))
          (bind _outoverlappingactors (Class|AuraAbilitySystemBPLibrary|GetLivePlayersWithinRadius (Variables|Default|GetAvatarActor) (Utilities|Array|MakeArray (Variables|Default|GetAvatarActor)) 45.0 _output_get_4))
          (for _array_element _outoverlappingactors
            (bind _returnvalue_5 (Class|CombatInterface|HasFriendlyFire(Message) (Variables|Default|GetAvatarActor)))
            (if _returnvalue_5
              (Class|AuraDamageGameplayAbility|CauseDamage _array_element :!label _label)
              (Variables|Default|SetHasHitTarget true)
              (elif (Class|AuraAbilitySystemBPLibrary|AreEnemies (Variables|Default|GetAvatarActor) _array_element)
                (goto _label))))
          (if (Variables|Default|GetHasHitTarget)
            (Class|GameplayAbility|ExecuteGameplayCuewithParams "(TagName=\"GameplayCue.MeleeImpact\")" (Ability|GameplayCue|MakeGameplayCueParameters :AggregatedSourceTags (GameplayTags|MakeGameplayTagContainerfromTag (.MontageTag (Utilities|Struct|BreakTaggedMontage (Variables|Default|GetTaggedMontage)))) :Location (Variables|Default|GetCombatSocketPos) :EffectCauser (Variables|Default|GetAvatarActor) :SourceObject (Variables|Default|GetCombatTarget))))
          (Ability|EndAbility))))
    (:OnCompleted
      (Ability|EndAbility :!label _label_2))
    (:OnInterrupted
      (goto _label_2))
    (:OnCancelled
      (goto _label_2))))